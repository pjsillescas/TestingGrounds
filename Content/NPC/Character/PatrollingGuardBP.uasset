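; PatrollingGuardBP is a guard NPC character with a configurable body color and an aiming state.
; SetBodyColor creates a dynamic instance of the mesh's first material, sets its BodyColor parameter from the Color variable, and reapplies it.
; It runs from both the Construction Script and BeginPlay, while SetAiming stores the Aiming flag.
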(event `self.ReceiveBeginPlay`
  (`self.SetBodyColor`))

(fn `SetAiming`
  (params (Aiming :type Boolean))
  (set `self.Aiming` Aiming)
  (return))

(fn `SetBodyColor`
  (locals (DynamicMaterial :type "MaterialInstanceDynamic Object Reference"))
  (bind _returnvalue (`PrimitiveComponent.CreateDynamicMaterialInstance` (`self.Mesh`) 0 (`|GetArrayItem` (`MeshComponent.GetMaterials` (`self.Mesh`))) "None"))
  (bind _output_get (set `local.DynamicMaterial` _returnvalue))
  (`MaterialInstanceDynamic.SetVectorParameterValue` _output_get "BodyColor" (`self.Color`))
  (`PrimitiveComponent.SetMaterial` (`self.Mesh`) 0 (`local.DynamicMaterial`)))

(fn `UserConstructionScript`
  (`self.SetBodyColor`))