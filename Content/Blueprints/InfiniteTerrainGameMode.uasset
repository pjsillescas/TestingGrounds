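; Game mode that builds a strip of terrain tiles for an infinite-terrain level when play begins.
; BeginPlay spawns ten TileBP actors in a loop, remembering the last one spawned.
; GetCurrentTransform returns that tile's attach location, or an origin transform for the first, so each tile chains onto the previous one.
; Only this initial batch is spawned here; Tick is unused.
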(event `self.ReceiveBeginPlay`
  (set `self.InitialTransform` (`KismetMathLibrary.MakeTransform` (0.0 0.0 0.0)))
  (for _ (range 10)
    (bind _transform (`self.GetCurrentTransform`))
    (bind _returnvalue (`|SpawnActorFromClass` "/Game/Levels/TileBP.TileBP_C" _transform "Undefined" "OverrideRootScale" null null))
    (set `self.Tile` _returnvalue)))

(fn `GetCurrentTransform`
  (returns (Transform :type "Transform Structure"))
  (locals (LocalTransform :type "Transform Structure"))
  (bind _tile (`self.Tile`))
  (`/Engine/EditorBlueprintResources/StandardMacros.IsValid` _tile
    (:`Is Valid`
      (set `local.LocalTransform` (`/Game/Levels/TileBP.GetAttachLocation` _tile)))
    (:`Is Not Valid`
      (set `local.LocalTransform` (`self.InitialTransform`))))
  (return (`local.LocalTransform`)))

(fn `UserConstructionScript`)