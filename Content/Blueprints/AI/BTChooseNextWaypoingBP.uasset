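; Behavior tree task that selects the next patrol waypoint for an AI-controlled pawn.
; It reads the patrol point array from the pawn, cast to ThirdPersonCharacter, and writes the point at the blackboard's next-waypoint index into the Waypoint key.
; It then advances that index with modulo wrapping, so the route loops, and finishes with success.
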(event `self.ReceiveExecuteAI`
  (params (OwnerController :type "AIController Object Reference") (ControlledPawn :type "Pawn Object Reference"))
  (`self.GetPatrolPoints` ControlledPawn)
  (bind _index (`self.SetWaypoint`))
  (`self.CycleIndex` _index)
  (`self.FinishExecute` true))

(fn `CycleIndex`
  (params (Index :type Integer))
  (`BTFunctionLibrary.SetBlackboardValueAsInt` (`self.NextWaypointIndex`) (mod (+ Index 1) (`KismetArrayLibrary.Array_Length` (`self.PatrolPoints`))))
  (return))

(fn `GetPatrolPoints`
  (params (Object :type "Object Object Reference"))
  (bind _asthird_person_character (cast `/Game/ThirdPersonCPP/Blueprints/ThirdPersonCharacter` Object)
    (:`then`
      (set `self.PatrolPoints` (`/Game/ThirdPersonCPP/Blueprints/ThirdPersonCharacter.PatrolPoints` _asthird_person_character)))
    (:`CastFailed`
      _))
  (return))

(fn `SetWaypoint`
  (returns (Index :type Integer))
  (bind _returnvalue (`BTFunctionLibrary.GetBlackboardValueAsInt` (`self.NextWaypointIndex`)))
  (`BTFunctionLibrary.SetBlackboardValueAsObject` (`self.Waypoint`) (`|GetArrayItem` (`self.PatrolPoints`) _returnvalue))
  (return _returnvalue))