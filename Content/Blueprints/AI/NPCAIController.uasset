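; AI controller for NPCs that starts patrol behavior by setting up the PatrolBB blackboard and running the PatrolBT behavior tree on BeginPlay.
; On possession it prints the pawn's name, cast as a ThirdPersonCharacter, for debugging.
; A helper function returns the location of the first TargetPoint found in the level, with no empty check.
; A FindPatrolRoute call sits unconnected and never runs.
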(event `self.ReceiveBeginPlay`
  (`self.UseBlackboard` "/Game/Blueprints/AI/PatrolBB.PatrolBB")
  (`self.RunBehaviorTree` "/Game/Blueprints/AI/PatrolBT.PatrolBT"))

(event `self.OnPossess`
  (params (PossessedPawn :type "Pawn Object Reference"))
  (`KismetSystemLibrary.PrintString` (`KismetStringLibrary.Concat_StrStr` "Possessing " (`KismetSystemLibrary.GetObjectName` (cast `/Game/ThirdPersonCPP/Blueprints/ThirdPersonCharacter` PossessedPawn :!pure true)))))

(fn `GetTargetPointLocation`
  (returns (ReturnValue :type "Vector Structure"))
  (bind _outactors (`GameplayStatics.GetAllActorsOfClass` "/Script/Engine.TargetPoint"))
  (return (`self.K2_GetActorLocation` (`|GetArrayItem` _outactors))))

(fn `UserConstructionScript`)