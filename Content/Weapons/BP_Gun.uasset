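; BP_Gun is a weapon Blueprint that fires for its Carrier at a rate limited by CooldownTime.
; Cooldown starts full on BeginPlay and counts up each Tick.
; While a valid Carrier has TriggerPulled set and the cooldown has elapsed, Tick calls Fire and resets the counter.
; A debug string prints after firing only if the gun itself is player pawn 0.
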(event `self.ReceiveBeginPlay`
  (set `self.Cooldown` (`self.CooldownTime`)))

(event `self.ReceiveTick`
  (params (DeltaSeconds :type "Float (single-precision)"))
  (bind _carrier (`self.Carrier`))
  (set `self.Cooldown` (+ DeltaSeconds (`self.Cooldown`)))
  (`/Engine/EditorBlueprintResources/StandardMacros.IsValid` _carrier
    (:`Is Valid`
      (if (and (`/Game/Character/Character/BP_Character.TriggerPulled` _carrier) (>= (`self.Cooldown`) (`self.CooldownTime`)))
        (`self.Fire`)
        (set `self.Cooldown` 0.0)
        (if (== (`GameplayStatics.GetPlayerPawn` 0) self)
          (`KismetSystemLibrary.PrintString` "payunn"))))))

(fn `UserConstructionScript`)