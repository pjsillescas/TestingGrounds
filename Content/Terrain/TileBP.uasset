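; Endless-terrain tile with a gate that locks behind the player, requests the next tile and removes itself.
; Leaving LockingVolume on the gate's forward side turns the gate solid red and calls SpawnNewTile on InfiniteTerrainGameMode; re-entering from that side unlocks it to green.
; Side comes from a dot product against ArrowAttachPoint, whose transform GetAttachLocation exposes.
; Player overlap with GCVolume destroys the tile.
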(event `self.ReceiveBeginPlay`
  (`self.Unlock`))

(event `self.LockingVolume.OnComponentEndOverlap`
  (params (OverlappedComponent :type "PrimitiveComponent Object Reference") (OtherActor :type "Actor Object Reference") (OtherComp :type "PrimitiveComponent Object Reference") (OtherBodyIndex :type Integer))
  (`self.IsPlayer` OtherActor
    (:`then`
      (if (> (`self.GetPlayerDirection` OtherActor) 0.0)
        (`self.Lock`)
        (bind _asinfinite_terrain_game_mode (cast `/Game/Blueprints/InfiniteTerrainGameMode` (`GameplayStatics.GetGameMode`)))
        (`/Game/Blueprints/InfiniteTerrainGameMode.SpawnNewTile` _asinfinite_terrain_game_mode)))))

(event `self.LockingVolume.OnComponentBeginOverlap`
  (params (OverlappedComponent :type "PrimitiveComponent Object Reference") (OtherActor :type "Actor Object Reference") (OtherComp :type "PrimitiveComponent Object Reference") (OtherBodyIndex :type Integer) (bFromSweep :type Boolean) (SweepResult :type "HitResult Structure (by ref)"))
  (`self.IsPlayer` OtherActor
    (:`then`
      (if (> (`self.GetPlayerDirection` OtherActor) 0.0)
        (`self.Unlock`)))))

(event `self.GCVolume.OnComponentBeginOverlap`
  (params (OverlappedComponent :type "PrimitiveComponent Object Reference") (OtherActor :type "Actor Object Reference") (OtherComp :type "PrimitiveComponent Object Reference") (OtherBodyIndex :type Integer) (bFromSweep :type Boolean) (SweepResult :type "HitResult Structure (by ref)"))
  (`self.IsPlayer` OtherActor
    (:`then`
      (`self.K2_DestroyActor`))))

(fn `GetAttachLocation`
  (returns (AttachTransform :type "Transform Structure"))
  (return (`SceneComponent.K2_GetComponentToWorld` (`self.ArrowAttachPoint`))))

(fn `GetPlayerDirection`
  (params (Actor :type "Actor Object Reference"))
  (returns (Direction :type "Float (double-precision)"))
  (return (`KismetMathLibrary.Dot_VectorVector` (- (`self.K2_GetActorLocation` Actor) (`SceneComponent.K2_GetComponentLocation` (`self.StaticMeshGate`))) (`SceneComponent.GetForwardVector` (`self.ArrowAttachPoint`)))))

(fn `Lock`
  (bind _staticmeshgate (`self.StaticMeshGate`))
  (`PrimitiveComponent.SetCollisionEnabled` _staticmeshgate "QueryAndPhysics")
  (`PrimitiveComponent.SetMaterial` _staticmeshgate 0 "/Game/Terrain/RedBarrier.RedBarrier")
  (return))

(fn `Unlock`
  (bind _staticmeshgate (`self.StaticMeshGate`))
  (`PrimitiveComponent.SetCollisionEnabled` _staticmeshgate "NoCollision")
  (`PrimitiveComponent.SetMaterial` _staticmeshgate 0 "/Game/Terrain/GreenBarrier.GreenBarrier")
  (return))

(fn `UserConstructionScript`)